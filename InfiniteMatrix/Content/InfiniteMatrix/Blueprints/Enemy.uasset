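; Enemy actor that damages the player on impact and awards score when it hits anything else.
; A player hit destroys it, subtracts health, shows the blood splatter widget at half of 100 health or lower, and triggers death and restart at exactly zero.
; Any other hit destroys it and adds to the player's score.
; A Delay on Tick also destroys it after ten seconds.
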(event EventBeginPlay)

(event Collision|EventActorBeginOverlap
  (params (OtherActor :type Actor%20Object%20Reference)))

(event EventTick
  (params (DeltaSeconds :type Float%20%28single-precision%29))
  (Utilities|FlowControl|Delay 1e+01)
  (Actor|DestroyActor))

(event Collision|EventHit
  (params (MyComp :type Primitive%20Component%20Object%20Reference) (Other :type Actor%20Object%20Reference) (OtherComp :type Primitive%20Component%20Object%20Reference) (bSelfMoved :type Boolean) (HitLocation :type Vector :default "0, 0, 0") (HitNormal :type Vector :default "0, 0, 0") (NormalImpulse :type Vector :default "0, 0, 0") (Hit :type Hit%20Result%20Structure%20%28by%20ref%29))
  (bind _asbp_player (Utilities|Casting|CastToBP_Player Other)
    (:then
      (Actor|DestroyActor)
      (bind _output_get (Variables|/Game/InfiniteMatrix/Blueprints/BP_Player.BP_Player_C|SetCurrentHealth _asbp_player (- (Variables|/Game/InfiniteMatrix/Blueprints/BP_Player.BP_Player_C|GetCurrentHealth _asbp_player) 25.0)))
      (CallFunction|BloodSplatter _asbp_player)
      (if (== _output_get 0.0)
        (Variables|/Game/InfiniteMatrix/Blueprints/BP_Player.BP_Player_C|SetIsDead _asbp_player true)
        (Default|DisplayRestart _asbp_player)))
    (:CastFailed
      (Actor|DestroyActor)
      (bind _asbp_player_2 (Utilities|Casting|CastToBP_Player (Game|Player|GetPlayerPawn 0)))
      (Variables|/Game/InfiniteMatrix/Blueprints/BP_Player.BP_Player_C|SetScore _asbp_player_2 (+ (Variables|/Game/InfiniteMatrix/Blueprints/BP_Player.BP_Player_C|GetScore _asbp_player_2) 50)))))

(fn ConstructionScript)

(fn BloodSplatter
  (params (Player :type BP%20Player%20Object%20Reference))
  (if (<= (Variables|/Game/InfiniteMatrix/Blueprints/BP_Player.BP_Player_C|GetCurrentHealth Player) 5e+01)
    (UserInterface|Viewport|AddtoViewport (Variables|/Game/InfiniteMatrix/Blueprints/BP_Player.BP_Player_C|GetBloodSplatterRef Player) 0)))