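; Spawner actor that builds a chain of BP_Tunnel segments and randomly populates them with health packs and enemies.
; On BeginPlay it clears existing tunnels and bullets, then lays initial segments from the player's location, each at the previous one's SpawnPoint.
; Every segment receives a spawner reference and randomizes its wall.
; Each spawn also rolls chances for a pickup and an enemy at random offsets within it.
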(event EventBeginPlay
  (CallFunction|SpawnInitialTunnels))

(event Collision|EventActorBeginOverlap
  (params (OtherActor :type Actor%20Object%20Reference)))

(event EventTick
  (params (DeltaSeconds :type Float%20%28single-precision%29)))

(fn ConstructionScript)

(fn SpawnTunnel
  (params (SpawnLocation :type Vector))
  (Utilities|FlowControl|Sequence
    (:then_0
      (bind _returnvalue (Game|SpawnActorfromClass "/Game/InfiniteMatrix/Blueprints/BP_Tunnel.BP_Tunnel_C" (Math|Transform|MakeTransform SpawnLocation "0, 0, 0" "1,1,1") "Undefined" 0 0))
      (bind _output_get (Variables|Default|SetNewestTunnel _returnvalue))
      (Variables|/Game/InfiniteMatrix/Blueprints/BP_Tunnel.BP_Tunnel_C|SetTunnelSpawner _output_get self)
      (Default|RandomizeWall _output_get))
    (:then_1
      (CallFunction|SpawnHealthPack SpawnLocation))
    (:then_2
      (CallFunction|SpawnEnemy SpawnLocation))))

(fn SpawnTunnelatSpawnPoint
  (CallFunction|SpawnTunnel (Transformation|GetWorldLocation (Variables|/Game/InfiniteMatrix/Blueprints/BP_Tunnel.BP_Tunnel_C|GetSpawnPoint (Variables|Default|GetNewestTunnel)))))

(fn SpawnInitialTunnels
  (Utilities|FlowControl|Sequence
    (:then_0
      (bind _outactors (Actor|GetAllActorsOfClass "/Game/InfiniteMatrix/Blueprints/BP_Tunnel.BP_Tunnel_C"))
      (for _array_element _outactors
        (Actor|DestroyActor _array_element)
        (bind _outactors_2 (Actor|GetAllActorsOfClass "/Game/InfiniteMatrix/Blueprints/BP_Bullet.BP_Bullet_C"))
        (for _array_element_2 _outactors_2
          (Actor|DestroyActor _array_element_2))))
    (:then_1
      (for _index (range 0 2)
        (Utilities|IsValid (Variables|Default|GetNewestTunnel)
          (:Is%20Valid
            (CallFunction|SpawnTunnelatSpawnPoint))
          (:Is%20Not%20Valid
            (CallFunction|SpawnTunnel (Transformation|GetActorLocation (Game|Player|GetPlayerPawn 0)))))))))

(fn SpawnHealthPack
  (params (SpawnLocation :type Vector))
  (if (== (Math|Random|RandomInteger 10) 0)
    (Game|SpawnActorfromClass "/Game/InfiniteMatrix/Blueprints/BP_HealthPack.BP_HealthPack_C" (Math|Transform|MakeTransform (+ (Math|Vector|MakeVector (Math|Conversions|ToFloat(Integer) (Math|Random|RandomIntegerinRange 500 2000)) (Math|Conversions|ToFloat(Integer) (Math|Random|RandomIntegerinRange -250 250)) (Math|Conversions|ToFloat(Integer) (Math|Random|RandomIntegerinRange -250 250))) SpawnLocation) "0, 0, 0" "1,1,1") "Undefined" 0 0)))

(fn SpawnEnemy
  (params (SpawnLocation :type Vector))
  (if (== (Math|Random|RandomInteger 5) 0)
    (Game|SpawnActorfromClass "/Game/InfiniteMatrix/Blueprints/Enemy.Enemy_C" (Math|Transform|MakeTransform (+ (Math|Vector|MakeVector (Math|Conversions|ToFloat(Integer) (Math|Random|RandomIntegerinRange 500 2000)) (Math|Conversions|ToFloat(Integer) (Math|Random|RandomIntegerinRange -250 250)) (Math|Conversions|ToFloat(Integer) (Math|Random|RandomIntegerinRange -250 250))) SpawnLocation) "0, 0, 0" "1,1,1") "Undefined" 0 0)))