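; BP_HealthPack is a spinning health pickup that heals BP_Player when touched.
; Tick rotates the HealthPack component around its roll axis at RotateSpeed, scaled by delta time.
; On player overlap, UpdateHealth adds a fixed amount only at or below a health threshold.
; The pack then destroys itself and removes the player's blood splatter widget, even when no health was added.
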(event OnComponentBeginOverlap(HealthPack)
  (params (OverlappedComponent :type Primitive%20Component%20Object%20Reference) (OtherActor :type Actor%20Object%20Reference) (OtherComp :type Primitive%20Component%20Object%20Reference) (OtherBodyIndex :type Integer) (bFromSweep :type Boolean) (SweepResult :type Hit%20Result%20Structure%20%28by%20ref%29))
  (bind _asbp_player (Utilities|Casting|CastToBP_Player OtherActor))
  (CallFunction|UpdateHealth _asbp_player)
  (Actor|DestroyActor)
  (Widget|RemovefromParent (Variables|/Game/InfiniteMatrix/Blueprints/BP_Player.BP_Player_C|GetBloodSplatterRef _asbp_player)))

(event EventBeginPlay)

(event EventTick
  (params (DeltaSeconds :type Float%20%28single-precision%29))
  (Transformation|AddLocalRotation (Variables|Default|GetHealthPack) (Math|Rotator|MakeRotator (* (Variables|Default|GetRotateSpeed) DeltaSeconds) 0.0 0.0) false false))

(fn ConstructionScript)

(fn UpdateHealth
  (params (Player :type BP%20Player%20Object%20Reference))
  (if (<= (Variables|/Game/InfiniteMatrix/Blueprints/BP_Player.BP_Player_C|GetCurrentHealth Player) 75.0)
    (Variables|/Game/InfiniteMatrix/Blueprints/BP_Player.BP_Player_C|SetCurrentHealth Player (+ (Variables|/Game/InfiniteMatrix/Blueprints/BP_Player.BP_Player_C|GetCurrentHealth Player) 25.0))))